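; BP_Monster_Tomato is a tomato monster that doubles as a named item and disappears once matched or let through a door.
; BeginPlay looks up its item info to fill the name widget, and the construction script tints a dynamic body material with BodyColor.
; A successful match on authority stops AI movement; this and CanEnterDoor both disable collision and start a short timer, apparently for HandleOnTimeDeath's notify-and-destroy.
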(event `self.ReceiveBeginPlay`
  (bind _outiteminfo (`WNoxBlueprintFunctionLibrary.FindItemInfo` (`.ItemKey` (break `WNoxItemInfo` (`self.ItemInfo`)))))
  (set `self.ItemInfo` _outiteminfo)
  (bind _asitem_name_text (cast `/Game/UMG/ItemNameText` (`WidgetComponent.GetUserWidgetObject` (`self.Widget`))))
  (`TextBlock.SetText` (`/Game/UMG/ItemNameText.NameText` _asitem_name_text) (`KismetTextLibrary.Conv_StringToText` (`.Name` (break `ItemInfoTableRow` (`.TableRowInfo` (break `WNoxItemInfo` (`self.ItemInfo`))))))))

(event `self.OnMatchItemResult`
  (params (bMatched :type Boolean))
  (if bMatched
    (`/Engine/EditorBlueprintResources/ActorMacros.Switch Has Authority`
      (:`Authority`
        (`self.SetActorEnableCollision` false)
        (`KismetSystemLibrary.K2_SetTimerDelegate` (`|CreateDelegate` :!event `HandleOnTimeDeath`) 0.5)
        (bind _returnvalue (`AIBlueprintHelperLibrary.GetAIController` self))
        (`Controller.StopMovement` _returnvalue)))))

(fn `CanEnterDoor`
  (returns (bCanEnter :type Boolean))
  (`KismetSystemLibrary.K2_SetTimerDelegate` (`|CreateDelegate` :!event `HandleOnTimeDeath`) 0.5)
  (`self.SetActorEnableCollision` false)
  (return true))

(fn `HandleOnTimeDeath`
  (`self.NotifyDisappear`)
  (`self.K2_DestroyActor`))

(fn `UserConstructionScript`
  (bind _mesh (`self.Mesh`))
  (bind _returnvalue (`PrimitiveComponent.CreateDynamicMaterialInstance` _mesh 0 (`PrimitiveComponent.GetMaterial` _mesh 0)))
  (bind _output_get (set `self.BodyMaterialInstance` _returnvalue))
  (`MaterialInstanceDynamic.SetVectorParameterValue` _output_get "BodyColor" (`self.BodyColor`)))