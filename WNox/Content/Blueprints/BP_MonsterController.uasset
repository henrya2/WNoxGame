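; BP_MonsterController is an AI controller that sends a possessed monster toward a door.
; On possession, on the server only, it initializes the MoveToTarget blackboard and finds all BP_Door actors.
; If any exist, it stores the first one as the target in the blackboard and runs the MoveToTarget behavior tree; otherwise the tree never starts.
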(event `self.OnPossess`
  (params (PossessedPawn :type "Pawn Object Reference"))
  (`/Engine/EditorBlueprintResources/ActorMacros.Switch Has Authority`
    (:`Authority`
      (bind _blackboardcomponent (`self.UseBlackboard` "/Game/BehaviorTrees/MoveToTarget_Blackboard.MoveToTarget_Blackboard"))
      (bind _output_get (set `self.NewBlackboardComp` _blackboardcomponent))
      (bind _outactors (`GameplayStatics.GetAllActorsOfClass` "/Game/Blueprints/BP_Door.BP_Door_C"))
      (if (`KismetArrayLibrary.Array_IsValidIndex` _outactors)
        (`BlackboardComponent.SetValueAsObject` (`self.NewBlackboardComp`) (`self.TargetName`) (`KismetArrayLibrary.Array_Get` _outactors))
        (`BlackboardComponent.SetValueAsObject` _output_get (`self.TargetName`) (`KismetArrayLibrary.Array_Get` _outactors))
        (`self.RunBehaviorTree` "/Game/BehaviorTrees/MoveToTarget_BT.MoveToTarget_BT")))))

(event `self.ReceiveBeginPlay`)

(fn `UserConstructionScript`)